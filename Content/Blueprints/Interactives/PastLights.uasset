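; PastLights is a time-vortex trigger that shifts the player into the past on capsule overlap, tinting post-processing and clearing IsPresent.
; Each instance registers an ID and queues it on the player controller; the first starts a timer with a UI throbber and clock sound.
; Each timeout pops the shared queue and restarts; once empty, the next hides and disables "Past"-tagged actors and restores the present.
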(event OnComponentBeginOverlap(Capsule)
  (params (OverlappedComponent :type Primitive%20Component%20Object%20Reference) (OtherActor :type Actor%20Object%20Reference) (OtherComp :type Primitive%20Component%20Object%20Reference) (OtherBodyIndex :type Integer) (bFromSweep :type Boolean) (SweepResult :type Hit%20Result%20Structure%20%28by%20ref%29))
  (bind _playercontroller (Variables|Default|GetPlayerController))
  (bind _vortexqueue (Variables|/Game/Mannequin/Character/Blueprints/ALS_Player_Controller.ALS_Player_Controller_C|GetVortexQueue _playercontroller))
  (if (not (Variables|Rendering|GetbHidden self))
    (Utilities|Casting|CastToPlayer_BP OtherActor)
    (Variables|/Game/Mannequin/Character/Blueprints/ALS_Player_Controller.ALS_Player_Controller_C|SetIsPresent (Variables|Default|GetPlayerController) false)
    (Utilities|Struct|SetmembersinPostProcessSettings (Variables|/Script/Engine.PostProcessVolume|GetSettings (Variables|Default|GetPostProcess)) -1.0)
    (Audio|PlaySound2D "/Game/Audio/Interactives/time_shift.time_shift" 1.0 1.0 0.0 0 0)
    (if (== (Utilities|Array|FindItem _vortexqueue (Variables|Default|GetVortexId)) -1)
      (if (and (== (Utilities|Array|Length (Variables|/Game/Mannequin/Character/Blueprints/ALS_Player_Controller.ALS_Player_Controller_C|GetVortexQueue (Variables|Default|GetPlayerController))) 0) (== (Variables|/Game/Mannequin/Character/Blueprints/ALS_Player_Controller.ALS_Player_Controller_C|GetIsTimeVortex (Variables|Default|GetPlayerController)) false))
        (Variables|/Game/Mannequin/Character/Blueprints/ALS_Player_Controller.ALS_Player_Controller_C|SetIsTimeVortex (Variables|Default|GetPlayerController) true)
        (Utilities|Array|Add (Variables|/Game/Mannequin/Character/Blueprints/ALS_Player_Controller.ALS_Player_Controller_C|GetVortexQueue (Variables|Default|GetPlayerController)) (Variables|Default|GetVortexId))
        (bind _foundwidgets (Widget|GetAllWidgetsOfClass "/Game/Blueprints/UI/WBP_MainUI.WBP_MainUI_C" false))
        (bind _returnvalue (UserInterface|CreateWidget "/Game/Blueprints/UI/CircularThrobber.CircularThrobber_C"))
        (Class|Widget|SetRenderTranslation _returnvalue "(X=20.000000,Y=800.000000)")
        (Class|CanvasPanel|AddChildtoCanvas (Variables|/Game/Blueprints/UI/WBP_MainUI.WBP_MainUI_C|GetCanvas (Utilities|Array|Get(acopy) _foundwidgets)) _returnvalue)
        (Audio|PlaySound2D (Variables|Default|GetClockSound) 1.0 1.0 0.0 0 0)
        (Utilities|Time|SetTimerbyEvent (delegate Custom|OnCycleTimer) 1e+01)
        (else
          (Utilities|Array|Add _vortexqueue (Variables|Default|GetVortexId))
          (Variables|/Game/Mannequin/Character/Blueprints/ALS_Player_Controller.ALS_Player_Controller_C|SetIsCounterX (Variables|Default|GetPlayerController) (> (Utilities|Array|Length (Variables|/Game/Mannequin/Character/Blueprints/ALS_Player_Controller.ALS_Player_Controller_C|GetVortexQueue (Variables|Default|GetPlayerController))) 1)))))))

(event OnComponentEndOverlap(Capsule)
  (params (OverlappedComponent :type Primitive%20Component%20Object%20Reference) (OtherActor :type Actor%20Object%20Reference) (OtherComp :type Primitive%20Component%20Object%20Reference) (OtherBodyIndex :type Integer)))

(event Custom|OnCycleTimer
  (bind _playercontroller (Variables|Default|GetPlayerController))
  (bind _playercontroller_2 (Variables|Default|GetPlayerController))
  (bind _vortexqueue (Variables|/Game/Mannequin/Character/Blueprints/ALS_Player_Controller.ALS_Player_Controller_C|GetVortexQueue _playercontroller_2))
  (if (> (Utilities|Array|Length (Variables|/Game/Mannequin/Character/Blueprints/ALS_Player_Controller.ALS_Player_Controller_C|GetVortexQueue (Variables|Default|GetPlayerController))) 0)
    (Utilities|Array|RemoveIndex _vortexqueue (- (Utilities|Array|Length _vortexqueue) 1))
    (Audio|PlaySound2D (Variables|Default|GetTimeOutSound) 1.0 1.0 0.0 0 0)
    (Variables|/Game/Mannequin/Character/Blueprints/ALS_Player_Controller.ALS_Player_Controller_C|SetIsCounterX (Variables|Default|GetPlayerController) (>= (Utilities|Array|Length (Variables|/Game/Mannequin/Character/Blueprints/ALS_Player_Controller.ALS_Player_Controller_C|GetVortexQueue (Variables|Default|GetPlayerController))) 1))
    (Audio|PlaySound2D (Variables|Default|GetClockSound) 1.0 1.0 0.0 0 0)
    (Utilities|Time|SetTimerbyEvent (delegate Custom|OnCycleTimer) 1e+01)
    (else
      (bind _foundwidgets (Widget|GetAllWidgetsOfClass "/Game/Blueprints/UI/CircularThrobber.CircularThrobber_C" false))
      (for _array_element _foundwidgets
        (Widget|RemovefromParent _array_element))
      (bind _outactors (Actor|GetAllActorswithTag "Past"))
      (for _array_element_2 _outactors
        (Rendering|SetActorHiddenInGame _array_element_2 true)
        (Collision|SetActorEnableCollision _array_element_2 false)
        (Variables|/Game/Mannequin/Character/Blueprints/ALS_Player_Controller.ALS_Player_Controller_C|SetIsTimeVortex _playercontroller false)
        (Variables|/Game/Mannequin/Character/Blueprints/ALS_Player_Controller.ALS_Player_Controller_C|SetIsPresent _playercontroller true)
        (Audio|PlaySound2D "/Game/Audio/Player/present_truth_sfx.present_truth_sfx" 1.0 1.0 0.0 0 0)
        (Utilities|Struct|SetmembersinPostProcessSettings (Variables|/Script/Engine.PostProcessVolume|GetSettings (Variables|Default|GetPostProcess)) 0.0 (Math|Vector4|MakeVector4 1.0 1.0 1.0 1.0))))))

(event EventBeginPlay
  (bind _returnvalue (Actor|GetActorOfClass "/Script/Engine.PostProcessVolume"))
  (Variables|Default|SetPostProcess _returnvalue)
  (bind _returnvalue_2 (Actor|GetActorOfClass "/Game/Mannequin/Character/Blueprints/ALS_Player_Controller.ALS_Player_Controller_C"))
  (bind _output_get (Variables|Default|SetPlayerController _returnvalue_2))
  (bind _output_get_2 (Variables|Default|SetVortexId (Utilities|Array|Length (Variables|/Game/Mannequin/Character/Blueprints/ALS_Player_Controller.ALS_Player_Controller_C|GetVortexIdentifiers _output_get))))
  (Utilities|Array|Add (Variables|/Game/Mannequin/Character/Blueprints/ALS_Player_Controller.ALS_Player_Controller_C|GetVortexIdentifiers _output_get) _output_get_2))

(fn ConstructionScript)