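; Player controller that owns the main UI, HP and mana, and drives a time-shift ability held on the A key.
; Shifting desaturates the level's post-process volume, plays a sound and sets visibility and collision on "Past"-tagged actors from IsTimeVortex; release reverts using IsPresent for tint.
; Tick drains or regenerates mana, forces release when empty, and slides the vortex-queue counter in and out.
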(event EventBeginPlay
  (bind _returnvalue (Actor|GetActorOfClass "/Script/Engine.PostProcessVolume"))
  (Variables|Default|SetPostProcess _returnvalue)
  (|ResetHP&Mana)
  (bind _returnvalue_2 (UserInterface|CreateWidget "/Game/Blueprints/UI/WBP_MainUI.WBP_MainUI_C"))
  (bind _output_get (Variables|Default|SetUI _returnvalue_2))
  (UserInterface|Viewport|AddtoViewport _output_get 0))

(event EventTick
  (params (DeltaSeconds :type Float%20%28single-precision%29))
  (bind _returnvalue (Math|Vector4|MakeVector4 1.0 1.0 1.0 1.0))
  (bind _returnvalue_2 (* DeltaSeconds 2.4e+02))
  (bind _postprocess (Variables|Default|GetPostProcess))
  (bind _ui (Variables|Default|GetUI))
  (bind _istimevortex (Variables|Default|GetIsTimeVortex))
  (bind _ui_2 (Variables|Default|GetUI))
  (bind _settings (Variables|/Script/Engine.PostProcessVolume|GetSettings _postprocess))
  (bind _manabar (Variables|/Game/Blueprints/UI/WBP_MainUI.WBP_MainUI_C|GetManaBar _ui))
  (bind _vortexcounter (Variables|/Game/Blueprints/UI/WBP_MainUI.WBP_MainUI_C|GetVortexCounter _ui_2))
  (bind _rendertransform (Variables|/Script/UMG.Widget|GetRenderTransform _vortexcounter))
  (bind _translation (Utilities|Struct|BreakWidgetTransform _rendertransform))
  (bind (_x _y) (Math|Vector2D|BreakVector2D _translation))
  (if (Variables|Default|GetIsCounterX)
    (Class|Widget|SetRenderTranslation _vortexcounter (Math|Vector2D|MakeVector2D _x (Math|Float|Clamp(Float) (- _y _returnvalue_2) -75.0 0.0)))
    (Variables|/Script/UMG.TextBlock|SetText _vortexcounter (Utilities|Text|ToText(String) (Utilities|String|Append (Utilities|String|ToString(Text) (Utilities|Text|ToText(Integer) (Utilities|Array|Length (Variables|Default|GetVortexQueue)))) "X")))
    (else
      (Class|Widget|SetRenderTranslation _vortexcounter (Math|Vector2D|MakeVector2D _x (Math|Float|Clamp(Float) (+ _returnvalue_2 _y) -75.0 0.0)))))
  (if (Variables|Default|GetIsTimeShift)
    (bind _output_get (Variables|Default|SetMana (- (Variables|Default|GetMana) (* DeltaSeconds 5e+01))))
    (Progress|SetPercent _manabar (/ _output_get (Variables|Default|GetManaMax)))
    (if (<= (/ _output_get (Variables|Default|GetManaMax)) 0.0)
      (Variables|Default|SetIsTimeShift false)
      (if (Variables|Default|GetIsPresent)
        (Utilities|Struct|SetmembersinPostProcessSettings _settings 0.0 _returnvalue)
        (else
          (Utilities|Struct|SetmembersinPostProcessSettings _settings -1.0 _returnvalue)))
      (Audio|PlaySound2D "/Game/Audio/Player/present_truth_sfx.present_truth_sfx" 1.0 1.0 0.0 0 0)
      (bind _outactors (Actor|GetAllActorswithTag "Past"))
      (for _array_element _outactors
        (Rendering|SetActorHiddenInGame _array_element (== _istimevortex false))
        (Collision|SetActorEnableCollision _array_element _istimevortex)))
    (else
      (bind _output_get_2 (Variables|Default|SetMana (+ (* DeltaSeconds 2e+01) (Variables|Default|GetMana))))
      (bind _output_get_3 (Variables|Default|SetMana (Math|Float|Clamp(Float) _output_get_2 0.0 (Variables|Default|GetManaMax))))
      (Progress|SetPercent _manabar (/ _output_get_3 (Variables|Default|GetManaMax))))))

(event Input|KeyboardEvents|A
  (params (Key :type Key%20Structure :default "None"))
  (bind _returnvalue (Math|Vector4|MakeVector4 1.0 1.0 1.0 1.0))
  (bind _postprocess (Variables|Default|GetPostProcess))
  (bind _istimevortex (Variables|Default|GetIsTimeVortex))
  (bind _istimevortex_2 (Variables|Default|GetIsTimeVortex))
  (bind _settings (Variables|/Script/Engine.PostProcessVolume|GetSettings _postprocess))
  (:Pressed
    (Variables|Default|SetIsTimeShift true)
    (Utilities|Struct|SetmembersinPostProcessSettings (Variables|/Script/Engine.PostProcessVolume|GetSettings (Variables|Default|GetPostProcess)) (Math|Vector4|MakeVector4 0.1 0.1 0.1 1.0))
    (Audio|PlaySound2D "/Game/Audio/Player/past_truth_sfx.past_truth_sfx" 1.0 1.0 0.0 0 0)
    (bind _outactors (Actor|GetAllActorswithTag "Past"))
    (for _array_element _outactors
      (Rendering|SetActorHiddenInGame _array_element _istimevortex_2)
      (Collision|SetActorEnableCollision _array_element (== _istimevortex_2 false))))
  (:Released
    (if (Variables|Default|GetIsTimeShift)
      (Variables|Default|SetIsTimeShift false)
      (if (Variables|Default|GetIsPresent)
        (Utilities|Struct|SetmembersinPostProcessSettings _settings 0.0 _returnvalue)
        (else
          (Utilities|Struct|SetmembersinPostProcessSettings _settings -1.0 _returnvalue)))
      (Audio|PlaySound2D "/Game/Audio/Player/present_truth_sfx.present_truth_sfx" 1.0 1.0 0.0 0 0)
      (bind _outactors_2 (Actor|GetAllActorswithTag "Past"))
      (for _array_element_2 _outactors_2
        (Rendering|SetActorHiddenInGame _array_element_2 (== _istimevortex false))
        (Collision|SetActorEnableCollision _array_element_2 _istimevortex)))))

(fn ConstructionScript)

(fn ChangeHP
  (params (HPValue :type Float%20%28double-precision%29))
  (Default|SetLifeBar (Variables|Default|GetUI) (+ (Math|Float|Clamp(Float) (Variables|Default|GetHP) 0.0 (Variables|Default|GetHPMax)) HPValue)))